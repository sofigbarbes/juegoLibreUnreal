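; Harvestable wood resource that gives the player wood on each Farmear press while they are in range.
; A Gate, opened when Jugador overlaps the Box and closed on any actor end overlap, filters the input.
; Each press calls AñadirMadera and raises Destruir, updating the widget's progress bar until the actor is destroyed at full.
; On box overlap, the widget turns once toward the player.
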(event `self.ReceiveBeginPlay`
  (`self.EnableInput` (`GameplayStatics.GetPlayerController` 0)))

(event `InputAction|Farmear` :consume false
  (params (Key :type "Key Structure" :default "AnyKey"))
  ;[1 1 1] Farmear
  (:`Pressed`
    (`/Engine/EditorBlueprintResources/StandardMacros.Gate` true :!label _label ; abierto si está en colision, cerrado si sale del rango de colision
      (:`Exit`
        (`|ExecutionSequence`
          (:`then_0`
            (set `self.Destruir` (+ (`self.Destruir`) 10.0))
            (if (== (`self.Destruir`) 100.0)
              (`self.K2_DestroyActor`)
              (else
                (bind _asdestruir (cast `/Game/HUDS/Destruir` (`WidgetComponent.GetUserWidgetObject` (`self.Widget`)))) ; actualizar estado destruir (%)
                (`ProgressBar.SetPercent` (`/Game/HUDS/Destruir.progreso_madera` _asdestruir) (/ (`self.Destruir`) 100.0)))))
          (:`then_1`
            (bind _asjugador (cast `/Game/Characters/Jugador` (`GameplayStatics.GetPlayerCharacter` 0)))
            (`/Game/Characters/Jugador.añadir madera` _asjugador)))))))

(event `self.Box.OnComponentBeginOverlap`
  (params (OverlappedComponent :type "PrimitiveComponent Object Reference") (OtherActor :type "Actor Object Reference") (OtherComp :type "PrimitiveComponent Object Reference") (OtherBodyIndex :type Integer) (bFromSweep :type Boolean) (SweepResult :type "HitResult Structure (by ref)"))
  ;[1 1 1] Farmear
  (`|ExecutionSequence`
    (:`then_0`
      (if (== (`GameplayStatics.GetObjectClass` OtherActor) "/Game/Characters/Jugador.Jugador_C")
        (goto _label :!via `Open`)))
    (:`then_1`
      (`SceneComponent.K2_SetWorldRotation` (`self.Widget`) (`KismetMathLibrary.FindLookAtRotation` (`SceneComponent.K2_GetComponentLocation` (`self.Widget`)) (`SceneComponent.K2_GetComponentLocation` (`Character.CapsuleComponent` (`GameplayStatics.GetPlayerCharacter` 0)))) false false) ; que la barra de progreso mire al jugador
    )))

(event `self.ReceiveActorEndOverlap`
  (params (OtherActor :type "Actor Object Reference"))
  ;[1 1 1] Farmear
  (`|ExecutionSequence`
    (:`then_0`
      (goto _label :!via `Close`))))

(fn `UserConstructionScript`)