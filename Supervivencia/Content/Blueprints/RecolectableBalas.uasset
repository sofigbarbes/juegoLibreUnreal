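; An ammo pickup actor that gives the Jugador player one bullet when overlapped.
; On overlap it plays the RECOGER_BALAS sound attached to its StaticMesh, destroys itself and increments the player's Balas count.
; A blocking hit from the Jugador also destroys the pickup, but that path plays no sound and adds no ammo.
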(event `self.ReceiveActorBeginOverlap`
  (params (OtherActor :type "Actor Object Reference"))
  (bind _asjugador (cast `/Game/Characters/Jugador` OtherActor))
  (`GameplayStatics.SpawnSoundAttached` "/Game/Sonidos/RECOGER_BALAS.RECOGER_BALAS" (`self.StaticMesh`))
  (`|ExecutionSequence`
    (:`then_1`
      (`self.K2_DestroyActor`)
      (bind _result (`/Engine/EditorBlueprintResources/StandardMacros.IncrementInt` (`/Game/Characters/Jugador.Balas` _asjugador))
        (:`  `
          (set `/Game/Characters/Jugador.Balas` _result _asjugador))))))

(event `self.ReceiveHit`
  (params (MyComp :type "PrimitiveComponent Object Reference") (Other :type "Actor Object Reference") (OtherComp :type "PrimitiveComponent Object Reference") (bSelfMoved :type Boolean) (HitLocation :type "Vector Structure") (HitNormal :type "Vector Structure") (NormalImpulse :type "Vector Structure") (Hit :type "HitResult Structure (by ref)"))
  (cast `/Game/Characters/Jugador` Other)
  (`self.K2_DestroyActor`))

(fn `UserConstructionScript`)