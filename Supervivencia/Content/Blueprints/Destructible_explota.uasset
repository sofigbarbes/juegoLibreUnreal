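; Destructible explosive actor that blows up when hit by a Disparo projectile.
; On overlap with a projectile it plays an attached explosion sound and applies radial damage around the projectile's location, guarded by an IsBroken flag so it only triggers once.
; When its destructible component fractures, it spawns a poison-shatter particle effect; the trailing delay leads to nothing.
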(event `self.ReceiveActorBeginOverlap`
  (params (OtherActor :type "Actor Object Reference"))
  (bind _asdisparo (cast `/Game/Blueprints/Disparo` OtherActor))
  (if (not (`self.IsBroken`))
    (`KismetSystemLibrary.PrintString` "colision true")
    (`GameplayStatics.SpawnSoundAttached` "/Game/Sonidos/explosion.explosion" (`self.DestructibleComponent`))
    (`GameplayStatics.ApplyRadialDamage` 50.0 (`self.K2_GetActorLocation` _asdisparo) 800.0)
    (set `self.IsBroken` true)))

(event `self.DestructibleComponent.OnComponentFracture`
  (params (HitPoint :type "Vector Structure (by ref)") (HitDirection :type "Vector Structure (by ref)"))
  (`GameplayStatics.SpawnEmitterAtLocation` "/Game/InfinityBladeEffects/Effects/FX_Skill_Aura/P_Aura_Poison_Shatter_01.P_Aura_Poison_Shatter_01" (`SceneComponent.K2_GetComponentLocation` (`self.DestructibleComponent`)))
  (`KismetSystemLibrary.Delay` 3.0))

(fn `UserConstructionScript`)