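; Bomb actor that counts down from BeginPlay, then explodes with an impulse, particle effect, sound, radial damage and world camera shake.
; A delay loop decrements CuentaAtrasExplosion until negative; StartExplosion zeroes it, cutting the countdown short.
; Explode also calls the player's Impactado if the player overlaps the bomb, and again for each overlapping Npc_dialogue, so NPCs caught in the blast penalize the player.
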(event `self.ReceiveBeginPlay`
  ;[1 1 1] Cuenta atras explosion + camera shake
  (if (>= (`self.cuentaAtrasExplosion`) 0) :!label _label
    (`KismetSystemLibrary.Delay` 0.1)
    (bind _result (`/Engine/EditorBlueprintResources/StandardMacros.DecrementInt` (`self.cuentaAtrasExplosion`))
      (:`  `
        (set `self.cuentaAtrasExplosion` _result)
        (goto _label)))
    (else
      (`KismetSystemLibrary.PrintString` "exploded")
      (`self.Explode`)
      (`GameplayStatics.PlayWorldCameraShake` "/Game/shakingCamera.shakingCamera_C" (`self.K2_GetActorLocation` (`GameplayStatics.GetPlayerController` 0)) 0.0 9000.0))))

(event `Explode`
  ;[1 1 1] Explode: check player and NPC who should be alive
  (`RadialForceComponent.FireImpulse` (`self.RadialForce`))
  (`ActorComponent.Activate` (`self.explosionEffect`) false)
  (`GameplayStatics.PlaySoundAtLocation` "/Game/Sonidos/explosion_bomb__mp3cut_net_.explosion_bomb__mp3cut_net_" (`SceneComponent.K2_GetComponentLocation` (`self.SkeletalMeshComponent`)))
  (`GameplayStatics.ApplyRadialDamage` :`BaseDamage` 100.0 :`Origin` (`SceneComponent.K2_GetComponentLocation` (`self.RadialForce`)) :`DamageRadius` 800.0 :`DamageTypeClass` "/Script/Engine.DamageType" :`bDoFullDamage` true)
  (`|ExecutionSequence`
    (:`then_0`
      (bind _asjugador (cast `/Game/Characters/Jugador` (`GameplayStatics.GetPlayerCharacter` 0)))
      (if (`self.IsOverlappingActor` _asjugador)
        (bind _asjugador_2 (cast `/Game/Characters/Jugador` (`GameplayStatics.GetPlayerCharacter` 0)))
        (`/Game/Characters/Jugador.Impactado` _asjugador_2 100)))
    (:`then_1`
      (bind _outactors (`GameplayStatics.GetAllActorsOfClass` "/Game/Characters/NPC_Dialogue/npc_dialogue.npc_dialogue_C"))
      (for _array_element _outactors
        (if (`self.IsOverlappingActor` _array_element)
          (bind _asjugador_3 (cast `/Game/Characters/Jugador` (`GameplayStatics.GetPlayerCharacter` 0)))
          (`/Game/Characters/Jugador.Impactado` _asjugador_3 100))))))

(fn `startExplosion`
  (`KismetSystemLibrary.PrintString` "funcion")
  (if (>= (`self.cuentaAtrasExplosion`) 0)
    (`/Engine/EditorBlueprintResources/StandardMacros.DecrementInt` (`self.cuentaAtrasExplosion`)
      (:`  `
        (set `self.cuentaAtrasExplosion` 0)
        (`KismetSystemLibrary.PrintString` (`KismetStringLibrary.Conv_IntToString` (`self.cuentaAtrasExplosion`)))))))

(fn `UserConstructionScript`)